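; BP_Enemy is a top-down enemy that turns to face the player, takes bullet damage and tracks melee range.
; A self-calling Delay loop updates its yaw toward the player.
; Bullet overlaps apply damage, updating health, a viewport healthbar widget and debug health states, and setting IsSlain at zero.
; The Melee overlap volume toggles InMelee and zooms the player's camera in and out.
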(event OnComponentBeginOverlap(Capsule)
  (params (OverlappedComponent :type Primitive%20Component%20Object%20Reference) (OtherActor :type Actor%20Object%20Reference) (OtherComp :type Primitive%20Component%20Object%20Reference) (OtherBodyIndex :type Integer) (bFromSweep :type Boolean) (SweepResult :type Hit%20Result%20Structure%20%28by%20ref%29))
  ;[1 1 1] If hit with bullet
  (bind _asbp_bullet (Utilities|Casting|CastToBP_Bullet OtherActor))
  (Development|PrintString "ow!")
  (Actor|DestroyActor _asbp_bullet)
  (Game|Damage|ApplyDamage self 1e+01 0 0))

(event OnComponentBeginOverlap(Melee)
  (params (OverlappedComponent :type Primitive%20Component%20Object%20Reference) (OtherActor :type Actor%20Object%20Reference) (OtherComp :type Primitive%20Component%20Object%20Reference) (OtherBodyIndex :type Integer) (bFromSweep :type Boolean) (SweepResult :type Hit%20Result%20Structure%20%28by%20ref%29))
  ;[1 1 1] Camera zoom
  (bind _asbp_top_down_character (Utilities|Casting|CastToBP_TopDownCharacter OtherActor))
  (Default|Zoomin _asbp_top_down_character)
  (Variables|Default|SetinMelee true)
  (Development|PrintString "Melee"))

(event OnComponentEndOverlap(Melee)
  (params (OverlappedComponent :type Primitive%20Component%20Object%20Reference) (OtherActor :type Actor%20Object%20Reference) (OtherComp :type Primitive%20Component%20Object%20Reference) (OtherBodyIndex :type Integer))
  ;[1 1 1] Camera zoom
  (bind _asbp_top_down_character (Utilities|Casting|CastToBP_TopDownCharacter OtherActor))
  (Default|ZoomOut _asbp_top_down_character)
  (Variables|Default|SetinMelee false)
  (Development|PrintString "Ranged"))

(event Custom|FacePlayer
  ;[1 1 1] Always Face Player
  (Transformation|SetActorRotation (Math|Rotator|MakeRotator 0.0 0.0 (.yaw (Class|KismetMathLibrary|RInterptoConstant (Transformation|GetActorRotation) (Math|Rotator|FindLookatRotation (Transformation|GetActorLocation) (Transformation|GetActorLocation (Variables|Default|GetPlayer%20Ref))) (Utilities|Time|GetWorldDeltaSeconds) 1e+02))))
  (Utilities|FlowControl|Delay 0.001)
  (CallFunction|FacePlayer))

(event Custom|Health%20Level
  ;[1 1 1] Checks if enemy is on low or critical health
  (if (< (Variables|Default|GetCurrHealth) (/ (Variables|Default|GetMaxHealth) 4.0))
    (Development|PrintString "Critical Health")
    (elif (< (Variables|Default|GetCurrHealth) (/ (Variables|Default|GetMaxHealth) 2.0))
      (Development|PrintString "Low Health")
      (else
        (Development|PrintString "Healthy")))))

(event EventBeginPlay
  ;[1 1 1] Initialises game (sets current health, adds hud to game, initialises enemy healthbar, before setting references)
  (Variables|Default|SetCurrHealth (Variables|Default|GetMaxHealth))
  (bind _returnvalue (UserInterface|CreateWidget "/Game/TopDown/Blueprints/BPW_HUD.BPW_HUD_C" (Game|GetPlayerController 0)))
  (bind _output_get (Variables|Default|SetWidget _returnvalue))
  (UserInterface|Viewport|AddtoViewport _output_get 0)
  (Progress|SetPercent (Variables|/Game/TopDown/Blueprints/BPW_HUD.BPW_HUD_C|GetHealthbar _returnvalue) (Math|Float|SafeDivide (Variables|Default|GetMaxHealth) (Variables|Default|GetMaxHealth)))
  (bind _asbp_top_down_character (Utilities|Casting|CastToBP_TopDownCharacter (Game|GetPlayerCharacter 0)))
  (Variables|Default|SetPlayer%20Ref _asbp_top_down_character)
  (CallFunction|FacePlayer)
  (Variables|Default|SetisSlain false))

(event Game|Damage|EventAnyDamage
  (params (Damage :type Float%20%28single-precision%29) (DamageType :type Damage%20Type%20Object%20Reference) (InstigatedBy :type Controller%20Object%20Reference) (DamageCauser :type Actor%20Object%20Reference))
  ;[1 1 1] Health System that allows for healing
  (bind _output_get (Variables|Default|SetCurrHealth (- (Variables|Default|GetCurrHealth) Damage)))
  (CallFunction|HealthLevel)
  (Progress|SetPercent (Variables|/Game/TopDown/Blueprints/BPW_HUD.BPW_HUD_C|GetHealthbar (Variables|Default|GetWidget)) (Math|Float|SafeDivide _output_get (Variables|Default|GetMaxHealth)))
  (if (<= (Variables|Default|GetCurrHealth) 0.0)
    (Development|PrintString "I'm Dead")
    (Variables|Default|SetisSlain true)))

(fn ConstructionScript)